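; Refrigerator prop with a Door component, set up to be used by interacting with its door.
; Use sets an IsInUse flag when the hit bone is "Door", and StopUsing clears it.
; Tick checks the flag but does nothing with it.
; An open/close timeline that would drive the door's relative yaw is present but never triggered, so the door does not move.
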(event EventStopUsing
  (Variables|Default|SetIsInUse false))

(event EventTick
  (params (DeltaSeconds :type Float%20%28single-precision%29))
  (if (Variables|Default|GetIsInUse)
    _))

(event EventUse
  (params (BoneName :type Name))
  (if (Utilities|Name|Equal(Name) BoneName "Door")
    (Variables|Default|SetIsInUse true)))

(fn ConstructionScript)